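; Example actor that demonstrates the food cooking material, taking a meat mesh from raw through cooked to burnt.
; On BeginPlay it assigns a dynamic instance of MI_FoodMeat, then a timeline drives its CookProgression scalar.
; A Niagara effect activates once as smoke when progression reaches 0.7, and deactivates and resets below that.
; An unconnected snippet sketches deriving the same scalar from ingredient timers.
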(event `self.ReceiveBeginPlay`
  ;[1 1 1] Creates dynamic material and assigns it to mesh - only needs to be done on begin play
  (bind _returnvalue (`KismetMaterialLibrary.CreateDynamicMaterialInstance` "/Game/Appartment/Shaders/Materials/Food/FoodCooking/MI_FoodMeat.MI_FoodMeat"))
  (`PrimitiveComponent.SetMaterial` (`self.StaticMesh`) 0 _returnvalue)
  ;[1 1 1] Timeline to show example for cooking
  (bind (_direction _cook) (`Timeline|Cook` :!via `PlayFromStart`)
    (:`Update`
      ;[1 1 1] Setting this value inside the dynamic material instance changes how cooked the material appears. 0 is raw, 0.5 is cooked, 1 is burnt.
      (`MaterialInstanceDynamic.SetScalarParameterValue` _returnvalue "CookProgression" _cook)
      ;[1 1 1] When timer hits .7 smoke starts then when the food hits 1 its burnt and the niagara system is deactivated
      (if (>= _cook 0.7)
        (`/Engine/EditorBlueprintResources/StandardMacros.DoOnce` false :!label _label
          (:`Completed`
            (`ActorComponent.Activate` (`self.Niagara`) false)))
        (else
          (`ActorComponent.Deactivate` (`self.Niagara`))
          (goto _label :!via `Reset`))))))

(fn `UserConstructionScript`)