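; BP_Hob is a cookware hob that tracks whether a pan is resting on it through a PanOn flag.
; On BeginPlay it stores the first BP_Pan found in the level as PanRef.
; Tick sets PanOn each frame from whether the Box overlaps any BP_Pan.
; A Sphere hit event also sets PanOn by checking the other actor's "Pan" tag, though Tick overwrites that value.
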(event `self.ReceiveBeginPlay`
  (bind _returnvalue (`GameplayStatics.GetActorOfClass` "/Game/Cookware/BP_Pan.BP_Pan_C"))
  (set `self.PanRef` _returnvalue))

(event `self.ReceiveTick`
  (params (DeltaSeconds :type "Float (single-precision)"))
  (if (> (`KismetArrayLibrary.Array_Length` (`PrimitiveComponent.GetOverlappingActors` (`self.Box`) "/Game/Cookware/BP_Pan.BP_Pan_C")) 0)
    (set `self.PanOn` true)
    (else
      (set `self.PanOn` false))))

(event `self.Sphere.OnComponentHit`
  (params (HitComponent :type "PrimitiveComponent Object Reference") (OtherActor :type "Actor Object Reference") (OtherComp :type "PrimitiveComponent Object Reference") (NormalImpulse :type "Vector Structure") (Hit :type "HitResult Structure (by ref)"))
  (if (`self.ActorHasTag` OtherActor "Pan")
    (set `self.PanOn` true)
    (else
      (set `self.PanOn` false))))

(fn `UserConstructionScript`)