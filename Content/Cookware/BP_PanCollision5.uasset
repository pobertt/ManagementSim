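; BP_PanCollision5 is a possessable cookware pan pawn that the first-person character can focus on and interact with.
; Focus calls toggle the outline's custom depth, flip the player's PanInteract flag and print a debug string.
; When possessed with that flag set, it stops movement and disables physics and collision.
; Pressing E repossesses the character, clears its pan-location timer and restores physics and collision.
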(event `self.ReceiveBeginPlay`
  (bind _returnvalue (`GameplayStatics.GetActorOfClass` "/Game/FirstPerson/Blueprints/BP_FirstPersonCharacter.BP_FirstPersonCharacter_C"))
  (set `self.PlayerRef` _returnvalue))

(event `self.ReceiveTick`
  (params (DeltaSeconds :type "Float (single-precision)")))

(event `Key|E`
  (params (Key :type "Key Structure"))
  (:`Pressed`
    (bind _returnvalue (`GameplayStatics.GetActorOfClass` "/Game/FirstPerson/Blueprints/BP_FirstPersonCharacter.BP_FirstPersonCharacter_C"))
    (`Controller.Possess` (`GameplayStatics.GetPlayerController` 0) _returnvalue)
    (`KismetSystemLibrary.K2_ClearAndInvalidateTimerHandle` (`/Game/FirstPerson/Blueprints/BP_FirstPersonCharacter.UpdatePanLocationTH` _returnvalue))
    (`PrimitiveComponent.SetConstraintMode` (`self._BoxComponent`) "Default")
    (`PrimitiveComponent.SetSimulatePhysics` (`self._BoxComponent`) true)
    (`PrimitiveComponent.SetCollisionEnabled` (`self._BoxComponent`) "QueryAndPhysics")))

(event `/Game/Interaction/BI_Interaction.Interface_ToggleFocus`
  (params (Focus :type Boolean))
  (`KismetSystemLibrary.PrintString` (`KismetStringLibrary.Conv_BoolToString` Focus) true true (struct :`R` 1.0 :`G` 0.722843 :`A` 1.0))
  (`PrimitiveComponent.SetRenderCustomDepth` (`self._MeshComponent`) Focus)
  (if (`/Game/FirstPerson/Blueprints/BP_FirstPersonCharacter.bPanInteract` (`self.PlayerRef`))
    (set `/Game/FirstPerson/Blueprints/BP_FirstPersonCharacter.bPanInteract` false (`self.PlayerRef`))
    (else
      (set `/Game/FirstPerson/Blueprints/BP_FirstPersonCharacter.bPanInteract` true (`self.PlayerRef`)))))

(event `self.ReceivePossessed`
  (params (NewController :type "Controller Object Reference"))
  (bind _playerref (`self.PlayerRef`))
  (`/Engine/EditorBlueprintResources/StandardMacros.IsValid` _playerref
    (:`Is Valid`
      (if (`/Game/FirstPerson/Blueprints/BP_FirstPersonCharacter.bPanInteract` _playerref)
        (`MovementComponent.StopMovementImmediately` (`self.FloatingPawnMovement`))
        (`PrimitiveComponent.SetSimulatePhysics` (`self._BoxComponent`) false)
        (`PrimitiveComponent.SetCollisionEnabled` (`self._BoxComponent`) "NoCollision")))))

(fn `GetInteractionWidgetRef`
  (returns (Ref :type "WidgetComponent Object Reference"))
  (return (`self.Widget`)))

(fn `UserConstructionScript`)