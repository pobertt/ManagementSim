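; BP_Carrot is a carrot ingredient that reacts to touching a hot cooking surface, with custom depth rendering enabled on its mesh.
; Mesh hits check actor tags: "Pan" counts only while the first BP_Hob found in the level has PanOn set, while "Hob" always counts.
; A valid hit applies a tiny impulse, waits a second, then calls OnHit, which is defined outside this graph.
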(event `self.ReceiveBeginPlay`
  (`PrimitiveComponent.SetRenderCustomDepth` (`self._MeshComponent`) true))

(event `self._MeshComponent.OnComponentHit`
  (params (HitComponent :type "PrimitiveComponent Object Reference") (OtherActor :type "Actor Object Reference") (OtherComp :type "PrimitiveComponent Object Reference") (NormalImpulse :type "Vector Structure") (Hit :type "HitResult Structure (by ref)"))
  (bind (_bblockinghit _binitialoverlap _time _distance _location _impactpoint _normal _impactnormal _physmat _hitactor) (`GameplayStatics.BreakHitResult` Hit))
  (`|ExecutionSequence`
    (:`then_0`
      (if (`self.ActorHasTag` _hitactor "Pan")
        (bind _returnvalue (`GameplayStatics.GetActorOfClass` "/Game/Cookware/BP_Hob.BP_Hob_C"))
        (if (`/Game/Cookware/BP_Hob.PanOn` _returnvalue)
          (`PrimitiveComponent.AddImpulse` (`self._MeshComponent`) (0.01 0.01 0.01) "None" false)
          (`KismetSystemLibrary.Delay` 1.0)
          (`self.OnHit`))))
    (:`then_1`
      (if (`self.ActorHasTag` _hitactor "Hob")
        (`PrimitiveComponent.AddImpulse` (`self._MeshComponent`) (0.01 0.01 0.01) "None" false)
        (`KismetSystemLibrary.Delay` 1.0)
        (`self.OnHit`)))))

(fn `UserConstructionScript`)