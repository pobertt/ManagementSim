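; Broccoli ingredient that cooks on contact with a switched-on pan or any hob-tagged actor.
; Hits nudge it with a tiny impulse, then call OnHit after a delay and notify the player if it has burned.
; Tick turns CookTime into progress for a dynamic material's CookProgression.
; Niagara activates at 70% progress; at full progress it stops and a scale timeline plays before the actor is destroyed.
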(event `self.ReceiveBeginPlay`
  (bind _returnvalue (`GameplayStatics.GetActorOfClass` "/Game/FirstPerson/Blueprints/BP_FirstPersonCharacter.BP_FirstPersonCharacter_C"))
  (set `self.PlayerRef` _returnvalue)
  ;[1 1 1] Material Handling
  (set `self.TotalTimer` (`self.CookTime`))
  (`PrimitiveComponent.SetRenderCustomDepth` (`self._MeshComponent`) true)
  ;;[1 1 1] Creates dynamic material and assigns it to mesh - only needs to be done on begin play
  (bind _returnvalue_2 (`KismetMaterialLibrary.CreateDynamicMaterialInstance` "/Game/Appartment/Shaders/Materials/Food/FoodCooking/MI_FoodVeggies.MI_FoodVeggies"))
  (`PrimitiveComponent.SetMaterial` (`self._MeshComponent`) 0 _returnvalue_2))

(event `self.ReceiveTick`
  (params (DeltaSeconds :type "Float (single-precision)"))
  (bind _returnvalue (+ (* (/ (`self.CookTime`) (`self.TotalTimer`)) -1.0) 1.0))
  ;[1 1 1] Material Handling
  (`MaterialInstanceDynamic.SetScalarParameterValue` (stale `self.ReceiveBeginPlay` _returnvalue_2) "CookProgression" _returnvalue)
  (if (>= _returnvalue 0.7)
    (if (>= _returnvalue 1.0)
      (`/Engine/EditorBlueprintResources/StandardMacros.DoOnce` false
        (:`Completed`
          (`ActorComponent.Deactivate` (`self.Niagara`))
          (bind (_direction _newtrack_0) (`Timeline|Timeline` :!via `PlayFromStart`)
            (:`Update`
              (`SceneComponent.SetWorldScale3D` (`self._MeshComponent`) (`KismetMathLibrary.VLerp` (0.0 0.0 0.0) (5.0 5.0 5.0) _newtrack_0)))
            (:`Finished`
              (`self.K2_DestroyActor`)))))
      (else
        (`/Engine/EditorBlueprintResources/StandardMacros.DoOnce` false
          (:`Completed`
            (`ActorComponent.Activate` (`self.Niagara`) false)))))))

(event `self._MeshComponent.OnComponentHit`
  (params (HitComponent :type "PrimitiveComponent Object Reference") (OtherActor :type "Actor Object Reference") (OtherComp :type "PrimitiveComponent Object Reference") (NormalImpulse :type "Vector Structure") (Hit :type "HitResult Structure (by ref)"))
  (bind (_bblockinghit _binitialoverlap _time _distance _location _impactpoint _normal _impactnormal _physmat _hitactor) (`GameplayStatics.BreakHitResult` Hit))
  (`|ExecutionSequence`
    (:`then_0`
      (if (`self.ActorHasTag` _hitactor "Pan")
        (bind _returnvalue (`GameplayStatics.GetActorOfClass` "/Game/Cookware/BP_Hob.BP_Hob_C"))
        (if (`/Game/Cookware/BP_Hob.PanOn` _returnvalue)
          (`PrimitiveComponent.AddImpulse` (`self._MeshComponent`) (0.01 0.01 0.01) "None" false)
          (`KismetSystemLibrary.Delay` 1.0)
          (`self.OnHit`)
          (if (`self.Burned`)
            (`/Game/FirstPerson/Blueprints/BP_FirstPersonCharacter.FoodBurnt` (`self.PlayerRef`))))))
    (:`then_1`
      (if (`self.ActorHasTag` _hitactor "Hob")
        (`PrimitiveComponent.AddImpulse` (`self._MeshComponent`) (0.01 0.01 0.01) "None" false)
        (`KismetSystemLibrary.Delay` 1.0)
        (`self.OnHit`)
        (if (`self.Burned`)
          (`/Game/FirstPerson/Blueprints/BP_FirstPersonCharacter.FoodBurnt` (`self.PlayerRef`)))))))

(fn `UserConstructionScript`)